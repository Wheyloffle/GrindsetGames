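; Campfire actor that takes souls from the player while they overlap it and uses them as fuel for its light.
; Each deposit moves one soul from the player's counter into the fire, spawns a wisp and sound, and resets the decay cooldown.
; After a starting delay, a BeginPlay loop drains the fuel until empty.
; SetLighting scales light radius and intensity exponentially with stored souls and permanently destroys the fire effect when nearly empty.
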(event Custom|Light%20Test%20Print%20Clock
  (Development|PrintString "Intensity:" :!label _label)
  (Development|PrintString (Utilities|String|ToString(Float) (Variables|/Script/Engine.LightComponentBase|GetIntensity (Variables|Default|GetPointLight))))
  (Development|PrintString "Radius:")
  (Development|PrintString (Utilities|String|ToString(Float) (Variables|/Script/Engine.LocalLightComponent|GetAttenuationRadius (Variables|Default|GetPointLight))))
  (Utilities|FlowControl|Delay 2.0)
  (goto _label))

(event Custom|Set%20Lighting
  (Rendering|Lighting|SetAttenuationRadius (Variables|Default|GetPointLight) (* (- (* (Math|Float|Power 1.02 (Variables|Default|GetSouls%20In%20Fire)) 2e+01) 2e+01) (Variables|Default|GetLight%20Radius%20Multiplier)))
  (Rendering|Components|Light|SetIntensity (Variables|Default|GetPointLight) (* (- (* (Math|Float|Power 1.02 (Variables|Default|GetSouls%20In%20Fire)) 2e+01) 2e+01) (Variables|Default|GetLight%20Intensity%20Multiplier)))
  (if (not (Variables|Default|GetFireDestroyed))
    (if (< (Variables|Default|GetSouls%20In%20Fire) 0.1)
      (Components|DestroyComponent (Variables|Default|GetP_Fire))
      (Variables|Default|SetFireDestroyed true))))

(event EventBeginPlay
  (CallFunction|SetLighting)
  (bind _asbp_first_person_character (Utilities|Casting|CastToBP_FirstPersonCharacter (Game|GetPlayerCharacter 0)))
  (bind _output_get (Variables|Default|SetPlayer%20Reference _asbp_first_person_character))
  ;[1 1 1] Initial Starting Delay before fire starts decaying
  (Utilities|FlowControl|Delay (Variables|Default|GetInitial%20Starting%20Delay%20Till%20Fire%20Decay))
  (if (> (Variables|Default|GetSouls%20In%20Fire) 0.0) :!label _label
    (if (< (Variables|Default|GetFireDecayCounter) 0.1)
      (Variables|Default|SetSouls%20In%20Fire (- (Variables|Default|GetSouls%20In%20Fire) (Variables|Default|GetSoul%20Decay%20Rate%20Per%20Seconds)))
      (else
        (Variables|Default|SetFireDecayCounter (- (Variables|Default|GetFireDecayCounter) 0.1))))
    (Utilities|FlowControl|Delay 0.1)
    (CallFunction|SetLighting)
    (goto _label)))

(event Collision|EventActorBeginOverlap
  (params (OtherActor :type Actor%20Object%20Reference))
  (if (== OtherActor (Variables|Default|GetPlayer%20Reference))
    (Variables|Default|SetIsOverlap true)
    (if (> (Variables|/Game/FirstPerson/Blueprints/BP_FirstPersonCharacter.BP_FirstPersonCharacter_C|GetSoulCounter (Variables|Default|GetPlayer%20Reference)) 0) :!label _label
      (Default|DecrementSoulCounter (Variables|Default|GetPlayer%20Reference))
      (Variables|Default|SetSouls%20In%20Fire (+ (Variables|Default|GetSouls%20In%20Fire) 1.0))
      (Game|SpawnActorfromClass "/Game/GameObjects/Campfire/BP_SoulWispEffect.BP_SoulWispEffect_C" (Math|Conversions|ToTransform(Vector) (+ (Transformation|GetWorldLocation (Variables|/Game/FirstPerson/Blueprints/BP_FirstPersonCharacter.BP_FirstPersonCharacter_C|GetLanternBox (Variables|Default|GetPlayer%20Reference))) "0,0,10.000000")) "Undefined" 0 0)
      (Audio|SpawnSound2D "/Game/Audio/SFX/SC_SoulDeposit.SC_SoulDeposit" 1.0 1.0 0.0 0)
      (Variables|Default|SetFireDecayCounter (Math|Conversions|ToFloat(Integer) (Variables|Default|GetSoul%20Sap%20Fire%20Decay%20Cooldown%20Time)))
      (Utilities|FlowControl|Delay (Math|Conversions|ToFloat(Integer) (/ 1 (Variables|Default|GetSouls%20To%20Sap%20Per%20Second))))
      (CallFunction|SetLighting)
      (if (Variables|Default|GetIsOverlap)
        (goto _label)))))

(event Collision|EventActorEndOverlap
  (params (OtherActor :type Actor%20Object%20Reference))
  (if (== OtherActor (Variables|Default|GetPlayer%20Reference))
    (Variables|Default|SetIsOverlap false)))

(fn ConstructionScript)