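; BP_SoulWispEffect is a soul wisp that flies into the campfire and adds one soul to it.
; On BeginPlay it finds the first BP_Campfire, starts a delayed Grow loop that steadily increases its scale, and eases its Arrow component to just above the fire.
; When the move completes it spawns BP_Explosion, destroys itself and increments the campfire's SoulsInFire count.
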(event Custom|Grow
  (Transformation|SetActorRelativeScale3D (Math|Vector|MakeVector (Variables|Default|GetScale) (Variables|Default|GetScale) (Variables|Default|GetScale)) :!label _label)
  (Utilities|FlowControl|Delay 0.05)
  (Variables|Default|SetScale (+ (Variables|Default|GetScale) 0.75))
  (if (> (Variables|Default|GetScale) 0.0)
    (goto _label)))

(event EventBeginPlay
  (bind _outactors (Actor|GetAllActorsOfClass "/Game/GameObject/Campfire/BP_Campfire.BP_Campfire_C"))
  (bind _output_get (Variables|Default|SetCampfire%20Object (Utilities|Array|Get(acopy) _outactors)))
  (CallFunction|Grow)
  (Components|MoveComponentTo (Variables|Default|GetArrow) (+ (Transformation|GetActorLocation _output_get) "0,0,20.000000") "0, 0, 0" false true 1.0 false)
  (Game|SpawnActorfromClass "/Game/GameObject/SoulPickUp/BP_Explosion.BP_Explosion_C" (Math|Transform|MakeTransform (Transformation|GetActorLocation) "0, 0, 0" "1.000000,1.000000,1.000000") "Undefined" 0 0)
  (Actor|DestroyActor)
  (Variables|/Game/GameObject/Campfire/BP_Campfire.BP_Campfire_C|SetSouls%20In%20Fire (Variables|Default|GetCampfire%20Object) (+ (Variables|/Game/GameObject/Campfire/BP_Campfire.BP_Campfire_C|GetSouls%20In%20Fire (Variables|Default|GetCampfire%20Object)) 1.0)))

(fn ConstructionScript)