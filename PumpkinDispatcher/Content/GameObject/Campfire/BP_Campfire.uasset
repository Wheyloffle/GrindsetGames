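; BP_Campfire is a campfire actor that drains souls from the first-person player while they overlap it.
; An overlap starts a delayed loop that decrements the player's SoulCounter, spawns a BP_SoulWisp at the player's transform and prints the count.
; The loop runs until the overlap ends or the souls run out.
; BeginPlay caches the player reference and also seeds its soul count.
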(event EventBeginPlay
  (bind _asbp_first_person_character (Utilities|Casting|CastToBP_FirstPersonCharacter (Game|GetPlayerCharacter 0)))
  (bind _output_get (Variables|Default|SetPlayer%20Reference _asbp_first_person_character))
  (Variables|/Game/FirstPerson/Blueprints/BP_FirstPersonCharacter.BP_FirstPersonCharacter_C|SetSoulCounter _output_get 100)
  (Variables|Default|SetIsOverlap false))

(event Collision|EventActorBeginOverlap
  (params (OtherActor :type Actor%20Object%20Reference))
  (bind _player_reference (Variables|Default|GetPlayer%20Reference))
  (if (== OtherActor _player_reference)
    (Variables|Default|SetIsOverlap true)
    (if (> (Variables|/Game/FirstPerson/Blueprints/BP_FirstPersonCharacter.BP_FirstPersonCharacter_C|GetSoulCounter _player_reference) 0) :!label _label
      (Variables|/Game/FirstPerson/Blueprints/BP_FirstPersonCharacter.BP_FirstPersonCharacter_C|SetSoulCounter (Variables|Default|GetPlayer%20Reference) (- (Variables|/Game/FirstPerson/Blueprints/BP_FirstPersonCharacter.BP_FirstPersonCharacter_C|GetSoulCounter _player_reference) 1))
      (Game|SpawnActorfromClass "/Game/GameObject/Campfire/BP_SoulWisp.BP_SoulWisp_C" (Transformation|GetActorTransform (Variables|Default|GetPlayer%20Reference)) "Undefined" 0 0)
      (Utilities|FlowControl|Delay 0.1)
      (Development|PrintString (Utilities|String|ToString(Integer) (Variables|/Game/FirstPerson/Blueprints/BP_FirstPersonCharacter.BP_FirstPersonCharacter_C|GetSoulCounter (Variables|Default|GetPlayer%20Reference))))
      (if (Variables|Default|GetIsOverlap)
        (goto _label)))))

(event Collision|EventActorEndOverlap
  (params (OtherActor :type Actor%20Object%20Reference))
  (if (== (Variables|Default|GetPlayer%20Reference) OtherActor)
    (Variables|Default|SetIsOverlap false)))

(fn ConstructionScript)