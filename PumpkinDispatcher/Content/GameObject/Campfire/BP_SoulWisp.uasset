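; BP_SoulWisp is a soul wisp that flies to the campfire and feeds it a soul.
; On BeginPlay it takes the first BP_Campfire found and eases its Arrow component to just above the fire's location with MoveComponentTo over a short time.
; It then destroys itself and increments the campfire's SoulsInFire count.
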(event EventBeginPlay
  (bind _outactors (Actor|GetAllActorsOfClass "/Game/GameObject/Campfire/BP_Campfire.BP_Campfire_C"))
  (bind _output_get (Variables|Default|SetCampfire%20Object (Utilities|Array|Get(acopy) _outactors)))
  (Components|MoveComponentTo (Variables|Default|GetArrow) (+ (Transformation|GetActorLocation _output_get) "0,0,20.000000") "100.000000, 0, 0" false true 1.0 false)
  (Actor|DestroyActor)
  (Variables|/Game/GameObject/Campfire/BP_Campfire.BP_Campfire_C|SetSoulsInFire (Variables|Default|GetCampfire%20Object) (+ (Variables|/Game/GameObject/Campfire/BP_Campfire.BP_Campfire_C|GetSoulsInFire (Variables|Default|GetCampfire%20Object)) 1.0)))

(event Collision|EventActorBeginOverlap
  (params (OtherActor :type Actor%20Object%20Reference)))

(event EventTick
  (params (DeltaSeconds :type Float%20%28single-precision%29)))

(fn ConstructionScript)