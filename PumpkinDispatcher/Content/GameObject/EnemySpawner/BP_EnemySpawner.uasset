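; Enemy spawner actor that spawns waves of BP_Thief around itself, growing more intense over time.
; After an initial delay, BeginPlay loops waves on a timed delay alongside an intensity clock that periodically raises the wave size limit.
; Each wave spawns a random count until done or the level-wide thief cap stops it.
; Spawn offsets use cosine and sine of random angles scaled by a radius, intended as a circle.
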(event Custom|Spawn%20Random%20Number%20Of%20Enemies
  (bind _returnvalue (Math|Random|RandomInteger 360))
  (bind _spawn_circle_radius (Variables|Default|GetSpawn%20Circle%20Radius))
  (bind _returnvalue_2 (Math|Conversions|ToFloat(Integer) _returnvalue))
  (Variables|Default|SetEnemies%20This%20Wave (+ (Math|Random|RandomInteger (Variables|Default|GetIntial%20Max%20Enemies%20Per%20Wave)) 1))
  (if (!= (Variables|Default|GetEnemies%20This%20Wave) 0) :!label _label
    (bind _outactors (Actor|GetAllActorsOfClass "/Game/GameObjects/Thief/BP_Thief.BP_Thief_C"))
    (if (<= (Utilities|Array|Length _outactors) (Variables|Default|GetMax%20Enemies%20In%20Level))
      (Game|SpawnActorfromClass "/Game/GameObjects/Thief/BP_Thief.BP_Thief_C" (Math|Conversions|ToTransform(Vector) (+ (Transformation|GetActorLocation) (Math|Vector|MakeVector (* (Math|Trig|Cos(Degrees) _returnvalue_2) _spawn_circle_radius) (* _spawn_circle_radius (Math|Trig|Sin(Degrees) _returnvalue_2)) 0.0))) "Undefined" 0 0)
      (Variables|Default|SetEnemies%20This%20Wave (- (Variables|Default|GetEnemies%20This%20Wave) 1))
      (goto _label))))

(event Custom|Start%20Intensity%20Clock
  (Utilities|FlowControl|Delay (Math|Conversions|ToFloat(Integer) (Variables|Default|GetTime%20Between%20Intesity%20Ramp%20Ups)) :!label _label)
  (Variables|Default|SetIntial%20Max%20Enemies%20Per%20Wave (+ (Variables|Default|GetIntial%20Max%20Enemies%20Per%20Wave) (Variables|Default|GetEnemies%20To%20Add%20Each%20Ramp%20Up)))
  (goto _label))

(event EventBeginPlay
  (Utilities|FlowControl|Delay (Variables|Default|GetTime%20Before%20First%20Spawn))
  (CallFunction|StartIntensityClock)
  (CallFunction|SpawnRandomNumberOfEnemies :!label _label)
  (Utilities|FlowControl|Delay (Variables|Default|GetSpawn%20Delay))
  (goto _label))

(fn ConstructionScript)