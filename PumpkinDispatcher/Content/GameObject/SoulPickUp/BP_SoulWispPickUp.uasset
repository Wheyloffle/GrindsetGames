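; Soul wisp pickup that bobs up and down while idle and turns on yaw to face the first-person player every tick.
; MoveSoulToLantern, not called within this Blueprint, eases the Arrow component to a supplied location while Shrink runs alongside it.
; Shrink prints a debug string, then steps the actor scale down in a Delay loop and destroys the actor at zero, independently of the move finishing.
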(event Custom|Begin%20Idle%20Animation
  (bind _wisp (Variables|Default|GetWisp))
  (bind _wisp_2 (Variables|Default|GetWisp))
  (bind _relativelocation (Variables|/Script/Engine.SceneComponent|GetRelativeLocation _wisp))
  (bind _relativelocation_2 (Variables|/Script/Engine.SceneComponent|GetRelativeLocation _wisp_2))
  (Components|MoveComponentTo (Variables|Default|GetWisp) (Math|Vector|MakeVector (.x _relativelocation_2) (.y _relativelocation_2) (+ (.z _relativelocation_2) 15.0)) "0, 0, 0" true true 1.0 false :!label _label)
  (Components|MoveComponentTo (Variables|Default|GetWisp) (Math|Vector|MakeVector (.x _relativelocation) (.y _relativelocation) (- (.z _relativelocation) 15.0)) "0, 0, 0" true true 1.0 false)
  (goto _label))

(event Custom|Move%20Soul%20To%20Lantern
  (params (Actor%20Location :type Vector))
  (CallFunction|Shrink)
  (Components|MoveComponentTo (Variables|Default|GetArrow) Actor%20Location "0.000000, 0, 0" true true (Variables|Default|GetTime%20It%20Takes%20To%20Move%20To%20The%20Lantern) false))

(event Custom|Shrink
  (Development|PrintString "AHAHHAHAHAHA")
  (Transformation|SetActorRelativeScale3D (Math|Vector|MakeVector (Variables|Default|GetScale) (Variables|Default|GetScale) (Variables|Default|GetScale)) :!label _label)
  (Utilities|FlowControl|Delay 0.05)
  (Variables|Default|SetScale (- (Variables|Default|GetScale) 0.1))
  (if (> (Variables|Default|GetScale) 0.0)
    (goto _label)
    (else
      (Actor|DestroyActor))))

(event EventBeginPlay
  (CallFunction|BeginIdleAnimation)
  (bind _asbp_first_person_character (Utilities|Casting|CastToBP_FirstPersonCharacter (Game|GetPlayerCharacter 0)))
  (Variables|Default|SetPlayer%20Character _asbp_first_person_character))

(event EventTick
  (params (DeltaSeconds :type Float%20%28single-precision%29))
  (Transformation|SetActorRotation (Math|Rotator|MakeRotator 0.0 0.0 (.yaw (Math|Rotator|FindLookatRotation (Transformation|GetActorLocation) (Transformation|GetActorLocation (Variables|Default|GetPlayer%20Character)))))))

(fn ConstructionScript)